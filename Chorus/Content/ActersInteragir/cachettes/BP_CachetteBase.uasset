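; Base hiding spot (wardrobe-style) the player can enter and leave, with outline and widget prompt when interaction is possible.
; Interaction toggles the player's hidden state, collision and movement, while timelines blend transform, view rotation and FOV and swing the door.
; Entering and exiting play sounds and emit noise through the player, and Tick accumulates time hidden on the player.
; The player's InteragirBloque dispatcher, bound at BeginPlay, also triggers the toggle until exit clears its bindings.
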(event Custom|Sortir
  (bind _as_bp_first_person_character (Variables|Default|GetAs%20BP%20First%20Person%20Character))
  (bind _exitpos (Variables|Default|GetexitPos))
  (bind _as_bp_first_person_character_2 (Variables|Default|GetAs%20BP%20First%20Person%20Character))
  (Variables|Default|Setjoueur%20cache false)
  ;[1 0.6767 0 0.5] Comment
  (Audio|PlaySound2D "/Game/ActersInteragir/cachettes/SE/OuvrirArmoire.OuvrirArmoire" 1.0 1.0 0.0 0 0)
  (Default|FaireSON (Variables|Default|GetAs%20BP%20First%20Person%20Character) 0.05 (Transformation|GetWorldLocation (Variables|Default|Getson)) false)
  (Variables|Default|Setprepos (Transformation|GetActorTransform _as_bp_first_person_character_2))
  (Utilities|FlowControl|Sequence
    (:then_0
      (bind (_direction _newtrack_0 _newtrack_1) (Timeline|Timeline_1 PlayFromStart)
        (:Update
          (Pawn|SetControlRotation (Game|GetPlayerController 0) (Math|Rotator|Lerp(Rotator) (Pawn|GetControlRotation (Game|GetPlayerController 0) :!class /Script/Engine.Controller) (Transformation|GetWorldRotation _exitpos) _newtrack_0 true))
          (Transformation|SetActorTransform _as_bp_first_person_character_2 (Math|Transform|Lerp(Transform) (Variables|Default|Getprepos) (Transformation|GetWorldTransform _exitpos) _newtrack_0))
          (Camera|SetFieldOfView (Variables|/Game/Player/BP_Player.BP_Player_C|GetFirstPersonCamera (Variables|Default|GetAs%20BP%20First%20Person%20Character)) (Math|Float|Lerp 7e+01 9e+01 _newtrack_1)))))
    (:then_1
      (Utilities|FlowControl|Delay 0.5)
      (Variables|Default|Setpeut%20preview true)
      (Variables|Default|SetPeutAppuyerE true)
      (Pawn|Components|CharacterMovement|SetMovementMode (Variables|/Script/Engine.Character|GetCharacterMovement _as_bp_first_person_character) "MOVE_Walking" 0)
      (Collision|SetCollisionEnabled (Variables|/Script/Engine.Character|GetCapsuleComponent _as_bp_first_person_character) "QueryAndPhysics")
      (Variables|/Game/Player/BP_Player.BP_Player_C|Setactionsbloquees (Variables|Default|GetAs%20BP%20First%20Person%20Character) false))))

(event Custom|InteragirBloque_Event
  (bind _as_bp_first_person_character (Variables|Default|GetAs%20BP%20First%20Person%20Character))
  (bind _capsulecomponent (Variables|/Script/Engine.Character|GetCapsuleComponent _as_bp_first_person_character))
  (if (Variables|Default|GetPeutAppuyerE)
    (Variables|Default|SetPeutAppuyerE false)
    (if (Variables|/Game/Player/BP_Player.BP_Player_C|Getest%20caché? _as_bp_first_person_character)
      (Variables|/Game/Player/BP_Player.BP_Player_C|Setest%20caché? _as_bp_first_person_character false)
      (Collision|SetCollisionEnabled _capsulecomponent "QueryAndPhysics")
      (Pawn|Components|CharacterMovement|DisableMovement (Variables|/Script/Engine.Character|GetCharacterMovement _as_bp_first_person_character))
      (CallFunction|Sortir)
      (CallFunction|OuvrirPorte)
      (EventDispatchers|UnbindallEventsfromInteragirBloque (stale EventBeginPlay _output_get))
      (else
        (Variables|/Game/Player/BP_Player.BP_Player_C|Setest%20caché? _as_bp_first_person_character true)
        (Collision|SetCollisionEnabled _capsulecomponent "NoCollision")
        (Pawn|Components|CharacterMovement|DisableMovement (Variables|/Script/Engine.Character|GetCharacterMovement _as_bp_first_person_character))
        (CallFunction|Rentrer)))))

(event Custom|coupereffet
  (Rendering|SetVisibility (Variables|Default|GetWidget) false false)
  (Rendering|Material|SetOverlayMaterial (Variables|Default|GetStaticMesh1) 0 :!class /Script/Engine.MeshComponent))

(event Custom|ouvrir%20porte
  (bind _newtrack_0 (Timeline|Timeline Reverse)
    (:Update
      (Transformation|SetRelativeRotation (Variables|Default|GetStaticMesh1) (Math|Rotator|MakeRotator 0.0 0.0 (Math|Float|Lerp 1.3e+02 0.0 _newtrack_0)) false false))))

(event Custom|fermer%20porte
  (bind _newtrack_0 (Timeline|Timeline Play)
    (:Update
      (Transformation|SetRelativeRotation (Variables|Default|GetStaticMesh1) (Math|Rotator|MakeRotator 0.0 0.0 (Math|Float|Lerp 1.3e+02 0.0 _newtrack_0)) false false))))

(event Custom|Rentrer
  (bind _playerpos (Variables|Default|GetPlayerPos))
  (Variables|/Game/Player/BP_Player.BP_Player_C|Setcache%20depuis%20x (Variables|Default|GetAs%20BP%20First%20Person%20Character) 0.0)
  (Variables|Default|Setjoueur%20cache true)
  ;[1 0.6767 0 0.5] Comment
  (Audio|PlaySound2D "/Game/ActersInteragir/cachettes/SE/FermerArmoire.FermerArmoire" 1.0 1.0 0.0 0 0)
  (Default|FaireSON (Variables|Default|GetAs%20BP%20First%20Person%20Character) 0.05 (Transformation|GetWorldLocation (Variables|Default|Getson)) false)
  (Variables|/Game/Player/BP_Player.BP_Player_C|Setactionsbloquees (Variables|Default|GetAs%20BP%20First%20Person%20Character) false)
  (Variables|Default|Setprepos (Transformation|GetActorTransform (Game|GetPlayerCharacter 0)))
  (Variables|Default|Setprerot (Pawn|GetControlRotation (Game|GetPlayerController 0) :!class /Script/Engine.Controller))
  (Utilities|FlowControl|Sequence
    (:then_0
      (bind (_direction _newtrack_0 _newtrack_1) (Timeline|Timeline_0 PlayFromStart)
        (:Update
          (Pawn|SetControlRotation (Game|GetPlayerController 0) (Math|Rotator|Lerp(Rotator) (Variables|Default|Getprerot) (Transformation|GetWorldRotation _playerpos) _newtrack_0 true))
          (Transformation|SetActorTransform (Variables|Default|GetAs%20BP%20First%20Person%20Character) (Math|Transform|Lerp(Transform) (Variables|Default|Getprepos) (Transformation|GetWorldTransform _playerpos) _newtrack_0))
          (Camera|SetFieldOfView (Variables|/Game/Player/BP_Player.BP_Player_C|GetFirstPersonCamera (Variables|Default|GetAs%20BP%20First%20Person%20Character)) (Math|Float|Lerp 9e+01 7e+01 _newtrack_1)))))
    (:then_1
      (Utilities|FlowControl|Delay 0.5)
      (Variables|Default|Setpeut%20preview false)
      (CallFunction|Coupereffet)
      (CallFunction|FermerPorte)
      (Variables|Default|SetPeutAppuyerE true))))

(event EventInteragir
  (bind _as_bp_first_person_character (Variables|Default|GetAs%20BP%20First%20Person%20Character))
  (bind _capsulecomponent (Variables|/Script/Engine.Character|GetCapsuleComponent _as_bp_first_person_character))
  (if (Variables|Default|GetPeutAppuyerE)
    (Variables|Default|SetPeutAppuyerE false)
    (if (Variables|/Game/Player/BP_Player.BP_Player_C|Getest%20caché? _as_bp_first_person_character)
      (Variables|/Game/Player/BP_Player.BP_Player_C|Setest%20caché? _as_bp_first_person_character false)
      (Collision|SetCollisionEnabled _capsulecomponent "QueryAndPhysics")
      (Pawn|Components|CharacterMovement|DisableMovement (Variables|/Script/Engine.Character|GetCharacterMovement _as_bp_first_person_character))
      (CallFunction|Sortir)
      (CallFunction|OuvrirPorte)
      (EventDispatchers|UnbindallEventsfromInteragirBloque (stale EventBeginPlay _output_get))
      (else
        (Variables|/Game/Player/BP_Player.BP_Player_C|Setest%20caché? _as_bp_first_person_character true)
        (Collision|SetCollisionEnabled _capsulecomponent "NoCollision")
        (Pawn|Components|CharacterMovement|DisableMovement (Variables|/Script/Engine.Character|GetCharacterMovement _as_bp_first_person_character))
        (CallFunction|Rentrer)))))

(event EventBeginPlay
  (bind _asbp_player (Utilities|Casting|CastToBP_Player (Game|GetPlayerCharacter 0)))
  (bind _output_get (Variables|Default|SetAs%20BP%20First%20Person%20Character _asbp_player))
  (EventDispatchers|AssignInteragirBloque _output_get (delegate Custom|InteragirBloque_Event)))

(event EventTick
  (params (DeltaSeconds :type Float%20%28single-precision%29))
  (bind _as_bp_first_person_character (Variables|Default|GetAs%20BP%20First%20Person%20Character))
  (if (Variables|Default|Getjoueur%20cache)
    (Variables|/Game/Player/BP_Player.BP_Player_C|Setcache%20depuis%20x _as_bp_first_person_character (+ (Variables|/Game/Player/BP_Player.BP_Player_C|Getcache%20depuis%20x _as_bp_first_person_character) (Utilities|Time|GetWorldDeltaSeconds)))))

(event EventInteractionPossible
  (params (PeutInteragirobjet :type Boolean))
  (if (Variables|Default|GetauthoriseUtilisation)
    (if PeutInteragirobjet
      (Variables|Default|SetPeutAppuyerE true)
      (if (Variables|Default|Getpeut%20preview)
        (Rendering|SetVisibility (Variables|Default|GetWidget) true false)
        (Rendering|Material|SetOverlayMaterial (Variables|Default|GetStaticMesh) "/Game/Player/Interaction/M_OutlineInteragir.M_OutlineInteragir" :!class /Script/Engine.MeshComponent))
      (else
        (Variables|Default|SetPeutAppuyerE false)
        (Rendering|SetVisibility (Variables|Default|GetWidget) false false)
        (Rendering|Material|SetOverlayMaterial (Variables|Default|GetStaticMesh1) 0 :!class /Script/Engine.MeshComponent)))))

(fn ConstructionScript
  (|CallParentFunction))