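; Base Blueprint for interactable actors that shows feedback when interaction with the object becomes possible.
; The InteractionPossible event, gated by AuthoriseUtilisation, toggles the PeutAppuyerE flag from its boolean input.
; When PeutPreview is set, becoming interactable also shows the Widget component and applies an outline overlay material to the StaticMesh.
; Losing interactability hides the widget and clears the overlay.
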(event EventInteractionPossible
  (params (PeutInteragirobjet :type Boolean))
  (if (Variables|Default|GetauthoriseUtilisation)
    (if PeutInteragirobjet
      (Variables|Default|SetPeutAppuyerE true)
      (if (Variables|Default|Getpeut%20preview)
        (Rendering|SetVisibility (Variables|Default|GetWidget) true false)
        (Rendering|Material|SetOverlayMaterial (Variables|Default|GetStaticMesh) "/Game/Player/Interaction/M_OutlineInteragir.M_OutlineInteragir" :!class /Script/Engine.MeshComponent))
      (else
        (Variables|Default|SetPeutAppuyerE false)
        (Rendering|SetVisibility (Variables|Default|GetWidget) false false)
        (Rendering|Material|SetOverlayMaterial (Variables|Default|GetStaticMesh) 0 :!class /Script/Engine.MeshComponent)))))

(fn ConstructionScript)