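; Base pickup item actor that the player can highlight and take into the left hand.
; When allowed, InteractionPossible sets the press-E flag and, if preview is enabled, shows a widget and outline overlay.
; A looping timer polls the player's HitActor and removes the highlight once it is no longer this item.
; Interagir plays a sound and passes the actor, mesh, padlock code and throwable flag to BP_Player.
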(event Custom|chechsur
  (if (not (== (Variables|/Game/Player/BP_Player.BP_Player_C|GetHit%20Actor (Variables|Default|GetAs%20BP%20First%20Person%20Character)) self))
    (Utilities|Time|ClearandInvalidateTimerbyHandle (stale Custom|lancer%20timer _returnvalue))
    (Rendering|SetVisibility (Variables|Default|GetWidget) false false)
    (Rendering|Material|SetOverlayMaterial (Variables|Default|GetStaticMesh) 0 :!class /Script/Engine.MeshComponent)))

(event Custom|lancer%20timer
  (bind _returnvalue (Utilities|Time|SetTimerbyEvent (delegate Custom|chechsur) 0.25 true)))

(event EventBeginPlay
  (bind _asbp_first_person_character (Utilities|Casting|CastToBP_Player (Game|GetPlayerCharacter 0)))
  (Variables|Default|SetAs%20BP%20First%20Person%20Character _asbp_first_person_character))

(event EventInteragir
  (if (Variables|Default|GetauthoriseUtilisation)
    (Audio|PlaySound2D "/Game/ActersInteragir/Items/SE/EquiperObjet.EquiperObjet" 1.0 1.0 0.0 0 0)
    (bind _asbp_first_person_character (Utilities|Casting|CastToBP_Player (Game|GetPlayerCharacter 0)))
    (Default|AjouterObjetMainGauche _asbp_first_person_character (Utilities|Struct|MakeObjetEnMain self (Variables|/Script/Engine.StaticMeshComponent|GetStaticMesh (Variables|Default|GetStaticMesh)) (Variables|Default|GetCODEcadenas) (Variables|Default|Getjetable?)))))

(event EventInteractionPossible
  (params (PeutInteragirobjet :type Boolean))
  (if (Variables|Default|GetauthoriseUtilisation)
    (if PeutInteragirobjet
      (Variables|Default|SetPeutAppuyerE true)
      (CallFunction|LancerTimer)
      (if (Variables|Default|Getpeut%20preview)
        (Rendering|SetVisibility (Variables|Default|GetWidget) true false)
        (Rendering|Material|SetOverlayMaterial (Variables|Default|GetStaticMesh) "/Game/Player/Interaction/M_OutlineInteragir.M_OutlineInteragir" :!class /Script/Engine.MeshComponent))
      (else
        (Variables|Default|SetPeutAppuyerE false)
        (Rendering|SetVisibility (Variables|Default|GetWidget) false false)
        (Rendering|Material|SetOverlayMaterial (Variables|Default|GetStaticMesh) 0 :!class /Script/Engine.MeshComponent)))))

(fn ConstructionScript
  (|CallParentFunction))