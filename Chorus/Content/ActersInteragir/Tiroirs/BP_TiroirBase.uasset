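; Base interactable drawer that the player can open, close, or unlock with a matching code from the held item.
; InteractionPossible toggles the prompt widget and outline overlay.
; Interagir either unlocks, plays a locked rattle timeline, or alternates open and close timelines through a FlipFlop, adding offsets to the mesh's current Y each update.
; Each outcome spawns a sound emitter and reports noise through the player's FaireSON.
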(event EventBeginPlay
  (bind _asbp_first_person_character (Utilities|Casting|CastToBP_Player (Game|GetPlayerCharacter 0)))
  (Variables|Default|SetAs%20BP%20First%20Person%20Character _asbp_first_person_character))

(event EventInteragir
  (bind _returnvalue (Transformation|GetActorTransform))
  (bind _returnvalue_2 (Transformation|GetActorTransform))
  (bind _staticmesh (Variables|Default|GetStaticMesh))
  (bind _staticmesh_2 (Variables|Default|GetStaticMesh))
  (bind _staticmesh_3 (Variables|Default|GetStaticMesh))
  (bind _relativelocation (Variables|/Script/Engine.SceneComponent|GetRelativeLocation _staticmesh_3))
  (bind _relativelocation_2 (Variables|/Script/Engine.SceneComponent|GetRelativeLocation _staticmesh))
  (bind _relativelocation_3 (Variables|/Script/Engine.SceneComponent|GetRelativeLocation _staticmesh_2))
  (if (Variables|Default|Getferme%20a%20clef?)
    (bind _asbp_first_person_character (Utilities|Casting|CastToBP_Player (Game|GetPlayerCharacter 0)))
    (if (Utilities|Enum|Equal(Enum) (Variables|/Game/Player/BP_Player.BP_Player_C|Getcodecadenasenmain _asbp_first_person_character) (Variables|Default|Getcodecadenas))
      (Audio|Components|Audio|Stop (Variables|Default|GetLockedtiroir))
      ;[1 0.6767 0 0.5] Comment
      (Variables|Default|Setferme%20a%20clef? false)
      (bind _returnvalue_3 (Game|SpawnActorfromClass "/Game/Audition/BP_EmmetteurDeSon.BP_EmmetteurDeSon_C" _returnvalue "Undefined" "MultiplyWithRoot" 0 0))
      (Default|SetSon _returnvalue_3 "/Game/ActersInteragir/Tiroirs/SE/ClefTiroir.ClefTiroir")
      (Default|JouerSon _returnvalue_3)
      ;[1 0.6767 0 0.5] Comment
      (Default|FaireSON (Variables|Default|GetAs%20BP%20First%20Person%20Character) 0.06 (Transformation|GetActorLocation) false :!label _label)
      (else
        (bind _returnvalue_4 (Game|SpawnActorfromClass "/Game/Audition/BP_EmmetteurDeSon.BP_EmmetteurDeSon_C" _returnvalue "Undefined" "MultiplyWithRoot" 0 0))
        (Default|SetSon _returnvalue_4 "/Game/ActersInteragir/Tiroirs/SE/TiroirFermAClef.TiroirFermAClef")
        (Default|JouerSon _returnvalue_4)
        (Utilities|FlowControl|Sequence
          (:then_0
            (goto _label))
          (:then_1
            (bind _newtrack_0 (Timeline|Lockedtiroir PlayFromStart)
              (:Update
                (Transformation|SetRelativeLocation (Variables|Default|GetStaticMesh) (Math|Vector|MakeVector (.x _relativelocation_2) (Math|Float|Lerp 0.0 2.5 _newtrack_0) (.z _relativelocation_2)) false false)))))))
    (else
      (Utilities|FlowControl|FlipFlop
        (:A
          ;[1 0.6767 0 0.5] Comment
          (bind _returnvalue_5 (Game|SpawnActorfromClass "/Game/Audition/BP_EmmetteurDeSon.BP_EmmetteurDeSon_C" _returnvalue_2 "Undefined" "MultiplyWithRoot" 0 0))
          (Default|SetSon _returnvalue_5 "/Game/ActersInteragir/Tiroirs/SE/ouvrirtiroir.ouvrirtiroir")
          (Default|JouerSon _returnvalue_5)
          (Default|FaireSON (Variables|Default|GetAs%20BP%20First%20Person%20Character) 0.06 (Transformation|GetActorLocation) false)
          (bind _newtrack_0_2 (Timeline|ouvrir PlayFromStart)
            (:Update
              (Transformation|SetRelativeLocation (Variables|Default|GetStaticMesh) (Math|Vector|MakeVector (.x _relativelocation_3) (+ (Math|Float|Lerp 0.0 1e+01 _newtrack_0_2) (.y _relativelocation_3)) (.z _relativelocation_3)) false false))))
        (:B
          (bind _returnvalue_6 (Game|SpawnActorfromClass "/Game/Audition/BP_EmmetteurDeSon.BP_EmmetteurDeSon_C" _returnvalue_2 "Undefined" "MultiplyWithRoot" 0 0))
          (Default|SetSon _returnvalue_6 "/Game/ActersInteragir/Tiroirs/SE/fermertiroir.fermertiroir")
          (Default|JouerSon _returnvalue_6)
          (Default|FaireSON (Variables|Default|GetAs%20BP%20First%20Person%20Character) 0.06 (Transformation|GetActorLocation) false)
          (bind _newtrack_0_3 (Timeline|Fermer PlayFromStart)
            (:Update
              (Transformation|SetRelativeLocation (Variables|Default|GetStaticMesh) (Math|Vector|MakeVector (.x _relativelocation) (+ (Math|Float|Lerp 0.0 -1e+01 _newtrack_0_3) (.y _relativelocation)) (.z _relativelocation)) false false))))))))

(event EventInteractionPossible
  (params (PeutInteragirobjet :type Boolean))
  (if (Variables|Default|GetauthoriseUtilisation)
    (if PeutInteragirobjet
      (Variables|Default|SetPeutAppuyerE true)
      (if (Variables|Default|Getpeut%20preview)
        (Rendering|SetVisibility (Variables|Default|GetWidget) true false)
        (Rendering|Material|SetOverlayMaterial (Variables|Default|GetStaticMesh) "/Game/Player/Interaction/M_OutlineInteragir.M_OutlineInteragir" :!class /Script/Engine.MeshComponent))
      (else
        (Variables|Default|SetPeutAppuyerE false)
        (Rendering|SetVisibility (Variables|Default|GetWidget) false false)
        (Rendering|Material|SetOverlayMaterial (Variables|Default|GetStaticMesh) 0 :!class /Script/Engine.MeshComponent)))))

(fn ConstructionScript
  (|CallParentFunction))