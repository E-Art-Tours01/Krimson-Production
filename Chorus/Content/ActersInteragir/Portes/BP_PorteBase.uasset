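; Base interactable door that the player or a monster can open, with outline and widget prompt, and that the player can listen through while closed.
; Interagir toggles timeline-driven rotation, swinging away from the opener, spawning sound emitters and reporting noise through the player.
; Interagir2 toggles listening: it locks the player's movement and actions, then blends position, view and FOV to the camera on their side, reversing the timeline to exit.
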(event Custom|fermer
  ;[1 0.6767 0 0.5] Comment
  (bind _returnvalue (Game|SpawnActorfromClass "/Game/Audition/BP_EmmetteurDeSon.BP_EmmetteurDeSon_C" (Transformation|GetActorTransform) "Undefined" "MultiplyWithRoot" 0 0))
  (Variables|Default|Setflipflopouvrir true)
  (Default|SetSon _returnvalue "/Game/ActersInteragir/Portes/SE/FermerPorte.FermerPorte")
  (Default|JouerSon _returnvalue)
  (Collision|SetCollisionEnabled (Variables|Default|GetPorte) "NoCollision")
  (Variables|Default|SetOuverte false)
  (Variables|Default|SetRelative%20Rotation%20Z%20%28Yaw%29 (.yaw (Variables|/Script/Engine.SceneComponent|GetRelativeRotation (Variables|Default|GetPorte))))
  (bind _newtrack_0 (Timeline|fermerporte PlayFromStart)
    (:Update
      (Transformation|SetRelativeRotation (Variables|Default|GetPorte) (Math|Rotator|MakeRotator 0.0 0.0 (Math|Float|Lerp (Variables|Default|GetRelative%20Rotation%20Z%20%28Yaw%29) 0.0 _newtrack_0)) false false))
    (:Finished
      (Collision|SetCollisionEnabled (Variables|Default|GetPorte) "QueryAndPhysics")
      (if (not (Variables|Default|GetOuverte))
        (Variables|Default|SetPossibled'ecouter true)))))

(event Custom|deplacer
  (bind _camerachoisie (Variables|Default|Getcamerachoisie))
  (bind _as_bp_first_person_character (Variables|Default|GetAs%20BP%20First%20Person%20Character))
  (Variables|Default|Setprepos (Transformation|GetActorTransform (Variables|Default|GetAs%20BP%20First%20Person%20Character)))
  (Variables|Default|Setprerot (Pawn|GetControlRotation (Game|GetPlayerController 0) :!class /Script/Engine.Controller))
  (bind (_direction _deplacement _vue) (Timeline|deplacement PlayFromStart)
    (:Update
      (Pawn|SetControlRotation (Game|GetPlayerController 0) (Math|Rotator|Lerp(Rotator) (Variables|Default|Getprerot) (Transformation|GetWorldRotation _camerachoisie) _deplacement true))
      (Transformation|SetActorTransform _as_bp_first_person_character (Math|Transform|Lerp(Transform) (Variables|Default|Getprepos) (Transformation|GetWorldTransform _camerachoisie) _deplacement))
      (Camera|SetFieldOfView (Variables|/Game/Player/BP_Player.BP_Player_C|GetFirstPersonCamera _as_bp_first_person_character) (Math|Float|Lerp 9e+01 7e+01 _vue)))))

(event Custom|sortir
  (bind _camerachoisie (Variables|Default|Getcamerachoisie))
  (bind _as_bp_first_person_character (Variables|Default|GetAs%20BP%20First%20Person%20Character))
  (bind (_direction _deplacement _vue) (Timeline|deplacement ReverseFromEnd)
    (:Update
      (Pawn|SetControlRotation (Game|GetPlayerController 0) (Math|Rotator|Lerp(Rotator) (Variables|Default|Getprerot) (Transformation|GetWorldRotation _camerachoisie) _deplacement true))
      (Transformation|SetActorTransform _as_bp_first_person_character (Math|Transform|Lerp(Transform) (Variables|Default|Getprepos) (Transformation|GetWorldTransform _camerachoisie) _deplacement))
      (Camera|SetFieldOfView (Variables|/Game/Player/BP_Player.BP_Player_C|GetFirstPersonCamera _as_bp_first_person_character) (Math|Float|Lerp 9e+01 7e+01 _vue)))))

(event Custom|retirer%20outline
  (Rendering|SetVisibility (Variables|Default|GetWidget) false false)
  (Rendering|Material|SetOverlayMaterial (Variables|Default|GetStaticMesh) 0 :!class /Script/Engine.MeshComponent)
  (Rendering|Material|SetOverlayMaterial (Variables|Default|GetPoignee2) 0 :!class /Script/Engine.MeshComponent))

(event Custom|arreterecoute_Event
  (bind _camera2 (Variables|Default|GetCamera2))
  (bind _camera1 (Variables|Default|GetCamera1))
  (bind _as_bp_first_person_character (Variables|Default|GetAs%20BP%20First%20Person%20Character))
  (if (not (Variables|Default|GetOuverte))
    (if (Variables|Default|GetPossibled'ecouter)
      (if (Variables|Default|Geteneciute)
        (Variables|/Game/Player/BP_Player.BP_Player_C|Setecoute%20porte _as_bp_first_person_character false)
        (Variables|Default|Seteneciute false)
        (Variables|Default|Setpeut%20preview true)
        (Variables|Default|SetPossibled'ecouter false)
        (CallFunction|Sortir)
        (Utilities|FlowControl|Delay 0.5)
        (Pawn|Components|CharacterMovement|SetMovementMode (Variables|/Script/Engine.Character|GetCharacterMovement (Variables|Default|GetAs%20BP%20First%20Person%20Character)) "MOVE_Walking" 0)
        (Variables|Default|SetPossibled'ecouter true)
        (Variables|/Game/Player/BP_Player.BP_Player_C|Setactionsbloquees (Variables|Default|GetAs%20BP%20First%20Person%20Character) false)
        (EventDispatchers|UnbindallEventsfromInteragirBloque (stale EventBeginPlay _output_get))
        (else
          (EventDispatchers|AssignInteragirBloque _as_bp_first_person_character (delegate Custom|arreterecoute_Event))
          (Variables|/Game/Player/BP_Player.BP_Player_C|Setecoute%20porte _as_bp_first_person_character true)
          (CallFunction|RetirerOutline)
          (Variables|/Game/Player/BP_Player.BP_Player_C|Setactionsbloquees (Variables|Default|GetAs%20BP%20First%20Person%20Character) true)
          (Variables|Default|Setpeut%20preview false)
          (Variables|Default|Seteneciute true)
          (Variables|Default|SetPossibled'ecouter false)
          (Pawn|Components|CharacterMovement|DisableMovement (Variables|/Script/Engine.Character|GetCharacterMovement (Variables|Default|GetAs%20BP%20First%20Person%20Character)))
          (if (> (Math|Vector|DotProduct (Transformation|GetActorForwardVector self) (Math|Vector|Normalize (- (Transformation|GetActorLocation (Variables|Default|GetAs%20BP%20First%20Person%20Character)) (Transformation|GetActorLocation self)))) 0.0)
            (Components|Activation|SetActive _camera2 false true)
            (Components|Activation|SetActive _camera1 true false)
            (Variables|Default|Setpositionsortie (Variables|Default|Getcote1))
            (Variables|Default|Setcamerachoisie (Variables|Default|GetCamera1))
            (else
              (Components|Activation|SetActive _camera2 true true)
              (Components|Activation|SetActive _camera1 false true)
              (Variables|Default|Setpositionsortie (Variables|Default|GetCote2))
              (Variables|Default|Setcamerachoisie (Variables|Default|GetCamera2))))
          (CallFunction|Deplacer)
          (Utilities|FlowControl|Delay 0.5)
          (Variables|Default|SetPossibled'ecouter true))))))

(event Custom|ouvrir
  (params (monstre :type Boolean) (Target :type Actor%20Object%20Reference))
  ;[1 0.6767 0 0.5] Comment
  (if monstre
    (Variables|Default|SetTarget Target)
    (else
      (Variables|Default|SetTarget (Game|GetPlayerCharacter 0))))
  (Variables|Default|Setflipflopouvrir false)
  (bind _returnvalue (Game|SpawnActorfromClass "/Game/Audition/BP_EmmetteurDeSon.BP_EmmetteurDeSon_C" (Transformation|GetActorTransform) "Undefined" "MultiplyWithRoot" 0 0))
  (Default|SetSon _returnvalue "/Game/ActersInteragir/Portes/SE/OuvrirPorte.OuvrirPorte")
  (Default|JouerSon _returnvalue)
  (Collision|SetCollisionEnabled (Variables|Default|GetPorte) "NoCollision")
  (Variables|Default|SetPossibled'ecouter false)
  (Variables|Default|SetOuverte true)
  (if (> (Math|Vector|DotProduct (Transformation|GetActorForwardVector self) (Math|Vector|Normalize (- (Transformation|GetActorLocation (Variables|Default|GetTarget)) (Transformation|GetActorLocation self)))) 0.0)
    (Variables|Default|SetRelative%20Rotation%20Z%20%28Yaw%29 (.yaw (Variables|/Script/Engine.SceneComponent|GetRelativeRotation (Variables|Default|GetPorte))))
    (bind _newtrack_0 (Timeline|Ouvrir1 PlayFromStart)
      (:Update
        (Transformation|SetRelativeRotation (Variables|Default|GetPorte) (Math|Rotator|MakeRotator 0.0 0.0 (Math|Float|Lerp (Variables|Default|GetRelative%20Rotation%20Z%20%28Yaw%29) -1.1e+02 _newtrack_0)) false false))
      (:Finished
        (Collision|SetCollisionEnabled (Variables|Default|GetPorte) "QueryAndPhysics")
        (if (not (Variables|Default|GetOuverte))
          (Variables|Default|SetPossibled'ecouter true))))
    (else
      (Variables|Default|SetRelative%20Rotation%20Z%20%28Yaw%29 (.yaw (Variables|/Script/Engine.SceneComponent|GetRelativeRotation (Variables|Default|GetPorte))))
      (bind _newtrack_0_2 (Timeline|ouvrir2 PlayFromStart)
        (:Update
          (Transformation|SetRelativeRotation (Variables|Default|GetPorte) (Math|Rotator|MakeRotator 0.0 0.0 (Math|Float|Lerp (Variables|Default|GetRelative%20Rotation%20Z%20%28Yaw%29) 1.1e+02 _newtrack_0_2)) false false))
        (:Finished
          (Collision|SetCollisionEnabled (Variables|Default|GetPorte) "QueryAndPhysics")
          (if (not (Variables|Default|GetOuverte))
            (Variables|Default|SetPossibled'ecouter true)))))))

(event EventBeginPlay
  (bind _asbp_first_person_character (Utilities|Casting|CastToBP_Player (Game|GetPlayerCharacter 0)))
  (bind _output_get (Variables|Default|SetAs%20BP%20First%20Person%20Character _asbp_first_person_character)))

(event EventInteragir
  (bind _returnvalue (Transformation|GetActorTransform))
  (bind _as_bp_first_person_character (Variables|Default|GetAs%20BP%20First%20Person%20Character))
  (bind _returnvalue_2 (Transformation|GetActorLocation _as_bp_first_person_character))
  (Audio|Components|Audio|Stop (Variables|Default|Getouvrir2))
  (if (Variables|Default|Getflipflopouvrir)
    ;[1 0.6767 0 0.5] Comment
    (Default|FaireSON _as_bp_first_person_character 0.06 _returnvalue_2 false)
    (Variables|Default|SetTarget (Game|GetPlayerCharacter 0))
    (Variables|Default|Setflipflopouvrir false)
    (bind _returnvalue_3 (Game|SpawnActorfromClass "/Game/Audition/BP_EmmetteurDeSon.BP_EmmetteurDeSon_C" _returnvalue "Undefined" "MultiplyWithRoot" 0 0))
    (Default|SetSon _returnvalue_3 "/Game/ActersInteragir/Portes/SE/OuvrirPorte.OuvrirPorte")
    (Default|JouerSon _returnvalue_3)
    (Collision|SetCollisionEnabled (Variables|Default|GetPorte) "NoCollision")
    (Variables|Default|SetPossibled'ecouter false)
    (Variables|Default|SetOuverte true)
    (if (> (Math|Vector|DotProduct (Transformation|GetActorForwardVector self) (Math|Vector|Normalize (- (Transformation|GetActorLocation (Variables|Default|GetTarget)) (Transformation|GetActorLocation self)))) 0.0)
      (Variables|Default|SetRelative%20Rotation%20Z%20%28Yaw%29 (.yaw (Variables|/Script/Engine.SceneComponent|GetRelativeRotation (Variables|Default|GetPorte))))
      (bind _newtrack_0 (Timeline|Ouvrir1 PlayFromStart)
        (:Update
          (Transformation|SetRelativeRotation (Variables|Default|GetPorte) (Math|Rotator|MakeRotator 0.0 0.0 (Math|Float|Lerp (Variables|Default|GetRelative%20Rotation%20Z%20%28Yaw%29) -1.1e+02 _newtrack_0)) false false))
        (:Finished
          (Collision|SetCollisionEnabled (Variables|Default|GetPorte) "QueryAndPhysics")
          (if (not (Variables|Default|GetOuverte))
            (Variables|Default|SetPossibled'ecouter true))))
      (else
        (Variables|Default|SetRelative%20Rotation%20Z%20%28Yaw%29 (.yaw (Variables|/Script/Engine.SceneComponent|GetRelativeRotation (Variables|Default|GetPorte))))
        (bind _newtrack_0_2 (Timeline|ouvrir2 PlayFromStart)
          (:Update
            (Transformation|SetRelativeRotation (Variables|Default|GetPorte) (Math|Rotator|MakeRotator 0.0 0.0 (Math|Float|Lerp (Variables|Default|GetRelative%20Rotation%20Z%20%28Yaw%29) 1.1e+02 _newtrack_0_2)) false false))
          (:Finished
            (Collision|SetCollisionEnabled (Variables|Default|GetPorte) "QueryAndPhysics")
            (if (not (Variables|Default|GetOuverte))
              (Variables|Default|SetPossibled'ecouter true))))))
    (else
      (Default|FaireSON _as_bp_first_person_character 0.06 _returnvalue_2 false)
      (bind _returnvalue_4 (Game|SpawnActorfromClass "/Game/Audition/BP_EmmetteurDeSon.BP_EmmetteurDeSon_C" _returnvalue "Undefined" "MultiplyWithRoot" 0 0))
      (Variables|Default|Setflipflopouvrir true)
      (Default|SetSon _returnvalue_4 "/Game/ActersInteragir/Portes/SE/FermerPorte.FermerPorte")
      (Default|JouerSon _returnvalue_4)
      (Collision|SetCollisionEnabled (Variables|Default|GetPorte) "NoCollision")
      (Variables|Default|SetOuverte false)
      (Variables|Default|SetRelative%20Rotation%20Z%20%28Yaw%29 (.yaw (Variables|/Script/Engine.SceneComponent|GetRelativeRotation (Variables|Default|GetPorte))))
      (bind _newtrack_0_3 (Timeline|fermerporte PlayFromStart)
        (:Update
          (Transformation|SetRelativeRotation (Variables|Default|GetPorte) (Math|Rotator|MakeRotator 0.0 0.0 (Math|Float|Lerp (Variables|Default|GetRelative%20Rotation%20Z%20%28Yaw%29) 0.0 _newtrack_0_3)) false false))
        (:Finished
          (Collision|SetCollisionEnabled (Variables|Default|GetPorte) "QueryAndPhysics")
          (if (not (Variables|Default|GetOuverte))
            (Variables|Default|SetPossibled'ecouter true)))))))

(event EventInteractionPossible
  (params (PeutInteragirobjet :type Boolean))
  (if (Variables|Default|GetauthoriseUtilisation)
    (if PeutInteragirobjet
      (Variables|Default|SetPeutAppuyerE true)
      (if (Variables|Default|Getpeut%20preview)
        (Rendering|SetVisibility (Variables|Default|GetWidget) true false)
        (Rendering|Material|SetOverlayMaterial (Variables|Default|GetStaticMesh) "/Game/Player/Interaction/M_OutlineInteragir.M_OutlineInteragir" :!class /Script/Engine.MeshComponent)
        (Rendering|Material|SetOverlayMaterial (Variables|Default|GetPoignee1) "/Game/Player/Interaction/M_OutlineInteragir.M_OutlineInteragir" :!class /Script/Engine.MeshComponent))
      (else
        (Variables|Default|SetPeutAppuyerE false)
        (Rendering|SetVisibility (Variables|Default|GetWidget) false false)
        (Rendering|Material|SetOverlayMaterial (Variables|Default|GetStaticMesh) 0 :!class /Script/Engine.MeshComponent)
        (Rendering|Material|SetOverlayMaterial (Variables|Default|GetPoignee2) 0 :!class /Script/Engine.MeshComponent)))))

(event EventInteragir2
  (bind _camera2 (Variables|Default|GetCamera2))
  (bind _camera1 (Variables|Default|GetCamera1))
  (bind _as_bp_first_person_character (Variables|Default|GetAs%20BP%20First%20Person%20Character))
  (if (not (Variables|Default|GetOuverte))
    (if (Variables|Default|GetPossibled'ecouter)
      (if (Variables|Default|Geteneciute)
        (Variables|/Game/Player/BP_Player.BP_Player_C|Setecoute%20porte _as_bp_first_person_character false)
        (Variables|Default|Seteneciute false)
        (Variables|Default|Setpeut%20preview true)
        (Variables|Default|SetPossibled'ecouter false)
        (CallFunction|Sortir)
        (Utilities|FlowControl|Delay 0.5)
        (Pawn|Components|CharacterMovement|SetMovementMode (Variables|/Script/Engine.Character|GetCharacterMovement (Variables|Default|GetAs%20BP%20First%20Person%20Character)) "MOVE_Walking" 0)
        (Variables|Default|SetPossibled'ecouter true)
        (Variables|/Game/Player/BP_Player.BP_Player_C|Setactionsbloquees (Variables|Default|GetAs%20BP%20First%20Person%20Character) false)
        (EventDispatchers|UnbindallEventsfromInteragirBloque (stale EventBeginPlay _output_get))
        (else
          (EventDispatchers|AssignInteragirBloque _as_bp_first_person_character (delegate Custom|arreterecoute_Event))
          (Variables|/Game/Player/BP_Player.BP_Player_C|Setecoute%20porte _as_bp_first_person_character true)
          (CallFunction|RetirerOutline)
          (Variables|/Game/Player/BP_Player.BP_Player_C|Setactionsbloquees (Variables|Default|GetAs%20BP%20First%20Person%20Character) true)
          (Variables|Default|Setpeut%20preview false)
          (Variables|Default|Seteneciute true)
          (Variables|Default|SetPossibled'ecouter false)
          (Pawn|Components|CharacterMovement|DisableMovement (Variables|/Script/Engine.Character|GetCharacterMovement (Variables|Default|GetAs%20BP%20First%20Person%20Character)))
          (if (> (Math|Vector|DotProduct (Transformation|GetActorForwardVector self) (Math|Vector|Normalize (- (Transformation|GetActorLocation (Variables|Default|GetAs%20BP%20First%20Person%20Character)) (Transformation|GetActorLocation self)))) 0.0)
            (Components|Activation|SetActive _camera2 false true)
            (Components|Activation|SetActive _camera1 true false)
            (Variables|Default|Setpositionsortie (Variables|Default|Getcote1))
            (Variables|Default|Setcamerachoisie (Variables|Default|GetCamera1))
            (else
              (Components|Activation|SetActive _camera2 true true)
              (Components|Activation|SetActive _camera1 false true)
              (Variables|Default|Setpositionsortie (Variables|Default|GetCote2))
              (Variables|Default|Setcamerachoisie (Variables|Default|GetCamera2))))
          (CallFunction|Deplacer)
          (Utilities|FlowControl|Delay 0.5)
          (Variables|Default|SetPossibled'ecouter true))))))

(fn ConstructionScript
  (|CallParentFunction))