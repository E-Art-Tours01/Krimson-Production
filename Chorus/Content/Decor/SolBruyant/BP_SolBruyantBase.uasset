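; Base actor for a noisy floor decor zone that gives away a player walking across it without crouching.
; A looping timer checks whether the player's capsule overlaps the Box while moving above a small speed threshold and standing.
; When triggered, it spawns a sound emitter at the player to play a random sound and calls the player's FaireSON to report noise at the zone's location.
; A Delay-reset flag imposes a cooldown between triggers.
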(event Custom|test
  (bind _asbp_first_person_character (Utilities|Casting|CastToBP_Player (Game|GetPlayerCharacter 0)))
  (if (Class|PrimitiveComponent|IsOverlappingComponent (Variables|Default|GetBox) (Variables|/Script/Engine.Character|GetCapsuleComponent _asbp_first_person_character))
    (if (Variables|Default|GetDelaiSon)
      (if (and (> (Math|Vector|VectorLength (Variables|/Script/Engine.MovementComponent|GetVelocity (Variables|/Script/Engine.Character|GetCharacterMovement _asbp_first_person_character))) 15.0) (not (Variables|/Game/Player/BP_Player.BP_Player_C|GetAccroupi? _asbp_first_person_character)))
        ;[1 0.6767 0 0.5] Comment
        (bind _returnvalue (Game|SpawnActorfromClass "/Game/Audition/BP_EmmetteurDeSon.BP_EmmetteurDeSon_C" (Transformation|GetActorTransform (Game|GetPlayerCharacter 0)) "Undefined" "MultiplyWithRoot" 0 0))
        (Default|SetSon _returnvalue (.OutItem (Utilities|Array|Random (Variables|Default|GetNew%20Sound))))
        (Default|JouerSon _returnvalue)
        (Default|FaireSON _asbp_first_person_character 1.0 (Transformation|GetActorLocation) false)
        (Variables|Default|SetDelaiSon false)
        (Utilities|FlowControl|Delay 5.0)
        (Variables|Default|SetDelaiSon true)))))

(event EventBeginPlay
  (Utilities|Time|SetTimerbyEvent (delegate Custom|test) 0.5 true))

(fn ConstructionScript)