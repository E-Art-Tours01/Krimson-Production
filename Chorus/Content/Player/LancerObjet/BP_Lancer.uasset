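; BP_Lancer is a thrown breakable object, apparently a bottle, that shatters and makes noise on impact.
; A looping timer caches the static mesh's physics velocity during flight.
; On hit, it spawns a glass-break sound emitter and reports a non-player noise through BP_Player.
; It then spawns a BP_bouteillecassable, passes it the cached velocity as direction, triggers its explosion and destroys itself.
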(event OnComponentHit(StaticMesh)
  (params (HitComponent :type Primitive%20Component%20Object%20Reference) (OtherActor :type Actor%20Object%20Reference) (OtherComp :type Primitive%20Component%20Object%20Reference) (NormalImpulse :type Vector :default "0, 0, 0") (Hit :type Hit%20Result%20Structure%20%28by%20ref%29))
  (bind _staticmesh (Variables|Default|GetStaticMesh))
  (bind _returnvalue (Transformation|GetWorldLocation _staticmesh))
  ;[0.15 0.15 0.15 0.5] Rebondir et spawn acteur
  (Utilities|Time|ClearandInvalidateTimerbyHandle (stale EventBeginPlay _returnvalue))
  ;;[1 0.6767 0 0.5] Comment
  (bind _returnvalue_2 (Game|SpawnActorfromClass "/Game/Audition/BP_EmmetteurDeSon.BP_EmmetteurDeSon_C" (Transformation|GetWorldTransform (Variables|Default|GetStaticMesh)) "AlwaysSpawn" "MultiplyWithRoot" 0 0))
  (Default|SetSon _returnvalue_2 "/Game/ActersInteragir/Items/Bouteilles/SE/VerreCasse.VerreCasse")
  (Default|JouerSon _returnvalue_2)
  (Default|FaireSON (Variables|Default|GetAs%20BP%20First%20Person%20Character) 1.0 _returnvalue false)
  (bind _returnvalue_3 (Game|SpawnActorfromClass "/Game/ActersInteragir/Items/Bouteilles/BP_bouteillecassable.BP_bouteillecassable_C" (Math|Transform|MakeTransform _returnvalue "0, 0, 0" "1.000000,1.000000,1.000000") "Undefined" "MultiplyWithRoot" 0 0))
  (Variables|/Game/ActersInteragir/Items/Bouteilles/BP_bouteillecassable.BP_bouteillecassable_C|Setdirection _returnvalue_3 (Variables|Default|Getvelocite))
  (Default|Exploser _returnvalue_3)
  (Actor|DestroyActor))

(event Custom|CustomEvent
  (bind _returnvalue (Physics|GetPhysicsLinearVelocity (Variables|Default|GetStaticMesh) "None"))
  (Variables|Default|Setvelocite _returnvalue))

(event EventBeginPlay
  (bind _asbp_first_person_character (Utilities|Casting|CastToBP_Player (Game|GetPlayerCharacter 0)))
  (Variables|Default|SetAs%20BP%20First%20Person%20Character _asbp_first_person_character)
  (CallFunction|CustomEvent)
  (bind _returnvalue (Utilities|Time|SetTimerbyEvent (delegate Custom|CustomEvent) 0.1 true)))

(fn ConstructionScript)