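; Ballerina enemy character that forces closed doors open on contact and jumpscares the player when its capsule overlaps theirs.
; A looping timer checks overlaps for doors, and the jumpscare fires once with a montage.
; SwitchTete toggles mouth and eyes states, changing light colour and playing or pausing music through a child sound emitter.
; Other events set walk-speed tiers and spawn or destroy an attached looping scream emitter.
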(event OnComponentBeginOverlap(Capsule)
  (params (OverlappedComponent :type Primitive%20Component%20Object%20Reference) (OtherActor :type Actor%20Object%20Reference) (OtherComp :type Primitive%20Component%20Object%20Reference) (OtherBodyIndex :type Integer) (bFromSweep :type Boolean) (SweepResult :type Hit%20Result%20Structure%20%28by%20ref%29))
  (bind _asbp_player (Utilities|Casting|CastToBP_Player OtherActor))
  (if (== (Variables|/Script/Engine.Character|GetCapsuleComponent _asbp_player) OtherComp)
    (Utilities|FlowControl|DoOnce false
      (:Completed
        (Variables|Default|Setjumpscaring true)
        (Transformation|SetActorRotation (Math|Rotator|FindLookatRotation (Transformation|GetActorLocation) (Transformation|GetActorLocation)))
        (Default|Jumpscare _asbp_player self)
        (Animation|Montage|PlayMontage (Variables|Character|GetMesh) "/Game/ENNEMY/anims/jumpsare.jumpsare"
          (:OnCompleted
            (Default|CallFini)))))))

(event Custom|ModeCri
  (Utilities|FlowControl|DoOnce false
    (:Completed
      (bind _returnvalue (Game|SpawnActorfromClass "/Game/Audition/BP_EmmetteurDeSon.BP_EmmetteurDeSon_C" (Math|Transform|MakeTransform (Transformation|GetWorldLocation (Variables|Default|GetpositionCRI)) "0, 0, 0" "1.000000,1.000000,1.000000") "Undefined" "MultiplyWithRoot" 0 0))
      (bind _output_get (Variables|Default|Setcriencours _returnvalue))
      (Variables|/Game/Audition/BP_EmmetteurDeSon.BP_EmmetteurDeSon_C|Setloop? _output_get true)
      (Default|SetSon (Variables|Default|Getcriencours) "/Game/ENNEMY/Ballerine/SE/crazy-distorted-screaming-sound-39350.crazy-distorted-screaming-sound-39350")
      (Default|JouerSon (Variables|Default|Getcriencours))
      (Transformation|AttachComponentToComponent (Variables|Default|Getcriencours) (Variables|Default|GetpositionCRI) "None" "SnapToTarget" "SnapToTarget" "SnapToTarget" true))))

(event Custom|resetcri
  (bind _criencours (Variables|Default|Getcriencours)
    (:then
      (Actor|DestroyActor _criencours)
      (Utilities|FlowControl|DoOnce false) ; enters at Reset
    )
    (:else)))

(event Custom|set%20moovespeed
  (params (moovespeed :type E_emoovespeeds%20Enum :default "NewEnumerator0"))
  (bind _charactermovement (Variables|Character|GetCharacterMovement))
  (switch Utilities|FlowControl|Switch|SwitchonE_emoovespeeds moovespeed
    (:NewEnumerator0
      (Variables|/Script/Engine.CharacterMovementComponent|SetMaxWalkSpeed _charactermovement 3e+02))
    (:NewEnumerator1
      (Variables|/Script/Engine.CharacterMovementComponent|SetMaxWalkSpeed _charactermovement 4.5e+02))
    (:NewEnumerator2
      (Variables|/Script/Engine.CharacterMovementComponent|SetMaxWalkSpeed _charactermovement 8e+02))))

(event Custom|SwitchTete
  (params (position :type E_etatTete%20Enum :default "NewEnumerator0"))
  (bind _as_bp_emmetteur_de_son (Variables|Default|GetAs%20BP%20Emmetteur%20De%20Son))
  (bind _pointlight (Variables|Default|GetPointLight))
  (if (not (Variables|Default|Getjumpscaring))
    (switch Utilities|FlowControl|Switch|SwitchonE_etatTete position
      (:NewEnumerator0
        (Rendering|Components|Light|SetLightColor _pointlight "(R=1.000000,G=0.065503,B=0.000000,A=1.000000)" true)
        (Default|JouerSon _as_bp_emmetteur_de_son))
      (:NewEnumerator1
        (Rendering|Components|Light|SetLightColor _pointlight "(R=0.000000,G=0.838710,B=1.000000,A=1.000000)" true)
        (Default|PauseSon _as_bp_emmetteur_de_son)))))

(event Custom|check%20contact
  (for _array_element (Collision|GetOverlappingActors (Variables|Default|GetCapsule) 0 :!class /Script/Engine.PrimitiveComponent)
    (bind _asbp_porte_base (Utilities|Casting|CastToBP_PorteBase _array_element))
    (if (not (Variables|/Game/ActersInteragir/Portes/BP_PorteBase.BP_PorteBase_C|GetOuverte _asbp_porte_base))
      (Default|Ouvrir _asbp_porte_base true self))))

(event EventBeginPlay
  (Utilities|Time|SetTimerbyFunctionName 0 "check contact" 0.1 true)
  (bind _asbp_emmetteur_de_son (Utilities|Casting|CastToBP_EmmetteurDeSon (Variables|/Script/Engine.ChildActorComponent|GetChildActor (Variables|Default|GetChildActor))))
  (bind _output_get (Variables|Default|SetAs%20BP%20Emmetteur%20De%20Son _asbp_emmetteur_de_son))
  (Default|SetSon _output_get "/Game/ENNEMY/Ballerine/SE/musiqueballerine.musiqueballerine")
  (Variables|/Game/Audition/BP_EmmetteurDeSon.BP_EmmetteurDeSon_C|Setloop? (Variables|Default|GetAs%20BP%20Emmetteur%20De%20Son) true))

(fn ConstructionScript)