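; BP_Maestro is a horror enemy that hunts the player with a metronome tick matching its slow, medium or running pace.
; Direct contact triggers a one-shot jumpscare, and a polling timer makes it force open closed doors.
; Its Check event catches players not holding their breath or recently hidden, sometimes feinting before opening the hiding spot.
; A freeze event temporarily halts movement and metronome, then signals resumption.
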(event Custom|Check
  (bind _catchingzone (Variables|Default|Getcatchingzone))
  (bind _as_bp_first_person_character (Variables|Default|GetAs%20BP%20First%20Person%20Character))
  ;[0.15 0.15 0.15 0.5] si deja attentif, cours
  (if (Variables|Default|Gettriggered?)
    (CallFunction|Moovespeed true false)
    (else
      (Variables|Default|Settriggered? true)))
  (for _array_element (Collision|GetOverlappingActors _catchingzone 0 :!class /Script/Engine.PrimitiveComponent)
    (Utilities|FlowControl|Sequence
      (:then_0
        (bind _asbp_player (Utilities|Casting|CastToBP_Player _array_element))
        (if (Class|PrimitiveComponent|IsOverlappingComponent _catchingzone (Variables|/Script/Engine.Character|GetCapsuleComponent _asbp_player))
          (if (not (Variables|/Game/Player/BP_Player.BP_Player_C|Getretiens%20respi _asbp_player))
            (if (< (Variables|/Game/Player/BP_Player.BP_Player_C|Geten%20respiration%20depuis _asbp_player) 3.0)
              (CallFunction|Jumpscare)))))
      (:then_1
        (bind _asbp_cachette_base (Utilities|Casting|CastToBP_CachetteBase _array_element))
        (Variables|Default|SetAs%20BP%20Cachette%20Base _asbp_cachette_base)
        (if (Variables|/Game/Player/BP_Player.BP_Player_C|Getest%20caché? _as_bp_first_person_character)
          (if (< (Variables|/Game/Player/BP_Player.BP_Player_C|Getcache%20depuis%20x _as_bp_first_person_character) 3.0)
            (Variables|Default|Setjs true)
            (CallFunction|Moovespeed false false)
            (AI|AIMoveTo self (Transformation|GetWorldLocation (Variables|/Game/ActersInteragir/cachettes/BP_CachetteBase.BP_CachetteBase_C|GetexitPos (Variables|Default|GetAs%20BP%20Cachette%20Base))) 0 15.0 false
              (:OnSuccess
                (Transformation|SetActorRotation (Math|Rotator|FindLookatRotation (Transformation|GetActorLocation) (Transformation|GetActorLocation (Variables|Default|GetAs%20BP%20First%20Person%20Character))))
                (Utilities|FlowControl|Delay 1.0)
                (CallFunction|SonEtonne)
                (if (> (Math|Random|RandomFloatinRange 0.0 15.0) 3.0)
                  (Default|OuvrirPorte (Variables|Default|GetAs%20BP%20Cachette%20Base))
                  (Utilities|FlowControl|Delay 0.5)
                  (CallFunction|Jumpscare)
                  (else
                    (AI|AIMoveTo self (Transformation|GetWorldLocation (Variables|/Game/ActersInteragir/cachettes/BP_CachetteBase.BP_CachetteBase_C|Getfeinte (Variables|Default|GetAs%20BP%20Cachette%20Base))) 0 5.0 false
                      (:OnSuccess
                        (Variables|/Game/ActersInteragir/BP_ActeurInteragirBase.BP_ActeurInteragirBase_C|SetPeutAppuyerE (Variables|Default|GetAs%20BP%20Cachette%20Base) false)
                        (AI|Navigation|StopMovement (AI|GetAIController self))
                        (Variables|/Script/Engine.CharacterMovementComponent|SetMaxWalkSpeed (Variables|Character|GetCharacterMovement) 4e+02)
                        (AI|AIMoveTo self (Transformation|GetWorldLocation (Variables|/Game/ActersInteragir/cachettes/BP_CachetteBase.BP_CachetteBase_C|GetexitPos (Variables|Default|GetAs%20BP%20Cachette%20Base))) 0 3.0 false
                          (:then
                            (Utilities|FlowControl|Delay 0.5)
                            (Default|OuvrirPorte (Variables|Default|GetAs%20BP%20Cachette%20Base))
                            (Utilities|FlowControl|Delay 0.2)
                            (CallFunction|Jumpscare))))))))))))))
  (Utilities|FlowControl|Delay 0.2)
  (if (not (Variables|Default|Getjs))
    (Default|CallFini)))

(event Custom|metronome%20vitesse%20moyen
  ;[0.15 0.15 0.15 0.5] metronome
  (bind _returnvalue (Utilities|Time|SetTimerbyEvent (delegate Custom|Bruit%20de%20metronome) 0.7 true))
  (Variables|Deplacement|Sethandle _returnvalue))

(event Custom|son%20etone%20delai
  (Utilities|FlowControl|Delay 3.0)
  (if (Math|Random|RandomBool)
    (Utilities|FlowControl|DoOnce false :!label _label
      (:Completed
        (bind _returnvalue (Game|SpawnActorfromClass "/Game/Audition/BP_EmmetteurDeSon.BP_EmmetteurDeSon_C" (Transformation|GetWorldTransform (Variables|Default|GetArrow1)) "Undefined" "MultiplyWithRoot" 0 0))
        (Default|SetSon _returnvalue (.OutItem (Utilities|Array|Random (Utilities|Array|MakeArray "/Game/ENNEMY/maestro/SE/maestroGemissement1.maestroGemissement1" "/Game/ENNEMY/maestro/SE/maestroGemissement2.maestroGemissement2" "/Game/ENNEMY/maestro/SE/maestroGemissement3.maestroGemissement3"))))
        (Default|JouerSon _returnvalue)
        (Utilities|FlowControl|Delay 2.0)
        (goto _label Reset)))))

(event Custom|Bruit%20de%20metronome
  ;[0.15 0.15 0.15 0.5] metronome
  (if (Variables|Deplacement|Getson%20metronome)
    (bind _returnvalue (Game|SpawnActorfromClass "/Game/Audition/BP_EmmetteurDeSon.BP_EmmetteurDeSon_C" (Transformation|GetWorldTransform (Variables|Default|GetArrow1)) "Undefined" "MultiplyWithRoot" 0 0))
    (Default|SetSon _returnvalue "/Engine/VREditor/Sounds/UI/Gizmo_Handle_Clicked.Gizmo_Handle_Clicked")
    (Default|JouerSon _returnvalue)))

(event Custom|jumpscare
  (Utilities|FlowControl|DoOnce false
    (:Completed
      (Transformation|SetActorRotation (Math|Rotator|FindLookatRotation (Transformation|GetActorLocation) (Transformation|GetActorLocation (Variables|Default|GetAs%20BP%20First%20Person%20Character))))
      (Default|Jumpscare (Variables|Default|GetAs%20BP%20First%20Person%20Character) self)
      (Animation|Montage|PlayMontage (Variables|Character|GetMesh) "/Game/ENNEMY/anims/jumpsare.jumpsare"
        (:OnCompleted
          (Default|CallFini))))))

(event Custom|Moovespeed
  (params (Run :type Boolean) (marchevite :type Boolean))
  (bind _charactermovement (Variables|Character|GetCharacterMovement))
  ;[0.15 0.15 0.15 0.5] moovespeed
  (if Run
    (Variables|/Script/Engine.CharacterMovementComponent|SetMaxWalkSpeed _charactermovement 5e+02)
    (if (not (Variables|Deplacement|Getrun?))
      (Utilities|Time|ClearandInvalidateTimerbyHandle (Variables|Deplacement|Gethandle))
      (Variables|Deplacement|Setrun? true)
      (Variables|Deplacement|Setwalk false)
      (Variables|deplacement|Setfastwalk? false)
      (CallFunction|MetronomeVitesseFast))
    (elif marchevite
      (Variables|/Script/Engine.CharacterMovementComponent|SetMaxWalkSpeed _charactermovement 3e+02)
      (if (not (Variables|deplacement|Getfastwalk?))
        (Utilities|Time|ClearandInvalidateTimerbyHandle (Variables|Deplacement|Gethandle))
        (Variables|deplacement|Setfastwalk? true)
        (Variables|Deplacement|Setrun? false)
        (Variables|Deplacement|Setwalk false)
        (CallFunction|MetronomeVitesseMoyen))
      (else
        (Variables|/Script/Engine.CharacterMovementComponent|SetMaxWalkSpeed _charactermovement 2e+02)
        (if (not (Variables|Deplacement|Getwalk))
          (Utilities|Time|ClearandInvalidateTimerbyHandle (Variables|Deplacement|Gethandle))
          (Variables|Deplacement|Setwalk true)
          (Variables|Deplacement|Setrun? false)
          (Variables|deplacement|Setfastwalk? false)
          (CallFunction|MetronomeVitessseLente))))))

(event Custom|check%20contact
  (for _array_element (Collision|GetOverlappingActors (Variables|Default|Getcatchingzonedirect) 0 :!class /Script/Engine.PrimitiveComponent)
    (bind _asbp_porte_base (Utilities|Casting|CastToBP_PorteBase _array_element))
    (if (not (Variables|/Game/ActersInteragir/Portes/BP_PorteBase.BP_PorteBase_C|GetOuverte _asbp_porte_base))
      (Default|Ouvrir _asbp_porte_base true self))))

(event Custom|Arretsur%20image
  (Components|Movement|StopMovementImmediately (Variables|Character|GetCharacterMovement))
  (AI|Navigation|StopMovement (AI|GetAIController self))
  (Variables|Deplacement|Setson%20metronome false)
  (Utilities|FlowControl|Delay 5.0)
  (Variables|Deplacement|Setson%20metronome true)
  (Default|CallRecommenceBouger))

(event Custom|metronome%20vitessse%20lente
  ;[0.15 0.15 0.15 0.5] metronome
  (bind _returnvalue (Utilities|Time|SetTimerbyEvent (delegate Custom|Bruit%20de%20metronome) 1.0 true))
  (Variables|Deplacement|Sethandle _returnvalue))

(event Custom|metronome%20vitesse%20fast
  ;[0.15 0.15 0.15 0.5] metronome
  (bind _returnvalue (Utilities|Time|SetTimerbyEvent (delegate Custom|Bruit%20de%20metronome) 0.35 true))
  (Variables|Deplacement|Sethandle _returnvalue))

(event Custom|SonEtonne
  (Utilities|FlowControl|DoOnce false :!label _label
    (:Completed
      (bind _returnvalue (Game|SpawnActorfromClass "/Game/Audition/BP_EmmetteurDeSon.BP_EmmetteurDeSon_C" (Transformation|GetWorldTransform (Variables|Default|GetArrow1)) "Undefined" "MultiplyWithRoot" 0 0))
      (Default|SetSon _returnvalue (.OutItem (Utilities|Array|Random (Utilities|Array|MakeArray "/Game/ENNEMY/maestro/SE/maestroGemissement1.maestroGemissement1" "/Game/ENNEMY/maestro/SE/maestroGemissement2.maestroGemissement2" "/Game/ENNEMY/maestro/SE/maestroGemissement3.maestroGemissement3"))))
      (Default|JouerSon _returnvalue)
      (Utilities|FlowControl|Delay 2.0)
      (goto _label Reset))))

(event EventBeginPlay
  (Utilities|Time|SetTimerbyFunctionName 0 "check contact" 0.1 true)
  (bind _asbp_player (Utilities|Casting|CastToBP_Player (Game|GetPlayerCharacter 0)))
  (Variables|Default|SetAs%20BP%20First%20Person%20Character _asbp_player)
  ;[0.15 0.15 0.15 0.5] metronome
  (bind _returnvalue (Utilities|Time|SetTimerbyEvent (delegate Custom|Bruit%20de%20metronome) 1.0 true))
  (Variables|Deplacement|Sethandle _returnvalue))

(event EventTick
  (params (DeltaSeconds :type Float%20%28single-precision%29))
  (if (Class|PrimitiveComponent|IsOverlappingComponent (Variables|Default|Getcatchingzonedirect) (Variables|/Script/Engine.Character|GetCapsuleComponent (Variables|Default|GetAs%20BP%20First%20Person%20Character)))
    (CallFunction|Jumpscare)))

(fn ConstructionScript)