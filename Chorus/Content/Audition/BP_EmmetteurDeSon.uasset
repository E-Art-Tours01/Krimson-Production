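; BP_EmmetteurDeSon is a sound emitter actor whose playback changes according to ear-based hearing states.
; It plays on BeginPlay with AutoLancement or through JouerSon, calling CheckSON on BP_Player beforehand.
; Right-ear, left-ear max and left-ear min events set the volume multiplier, with low-pass filtering only for left min.
; Loop replays finished audio; otherwise the actor destroys itself on finish or after a fixed delay.
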(event OnAudioFinished(Audio)
  (if (Variables|Default|Getloop?)
    (CallFunction|JouerSon)
    (else
      (Actor|DestroyActor))))

(event Custom|OreilleGaucheMIN
  (bind _audio (Variables|Default|GetAudio))
  (Audio|Components|Audio|SetVolumeMultiplier _audio 0.35 :!class /Script/Engine.AudioComponent)
  (Audio|Components|Audio|SetLowPassFilterEnabled _audio true :!class /Script/Engine.AudioComponent))

(event Custom|OreilleDroite
  (bind _audio (Variables|Default|GetAudio))
  (Audio|Components|Audio|SetVolumeMultiplier _audio 0.075 :!class /Script/Engine.AudioComponent)
  (Audio|Components|Audio|SetLowPassFilterEnabled _audio false :!class /Script/Engine.AudioComponent))

(event Custom|set%20Son
  (params (NewSound :type Sound%20Base%20Object%20Reference))
  (Audio|Components|Audio|SetSound (Variables|Default|GetAudio) NewSound))

(event Custom|OreilleGaucheMAX
  (bind _audio (Variables|Default|GetAudio))
  (Audio|Components|Audio|SetVolumeMultiplier _audio 1.0 :!class /Script/Engine.AudioComponent)
  (Audio|Components|Audio|SetLowPassFilterEnabled _audio false :!class /Script/Engine.AudioComponent))

(event Custom|pause%20son
  (Components|Activation|Deactivate (Variables|Default|GetAudio)))

(event Custom|JouerSon
  (bind _asbp_player (Utilities|Casting|CastToBP_Player (Game|GetPlayerCharacter 0))
    (:then
      (Default|CheckSON _asbp_player))
    (:CastFailed
      _))
  (Components|Activation|Activate (Variables|Default|GetAudio) false)
  (Utilities|FlowControl|Delay 15.0)
  (if (not (Variables|Default|Getloop?))
    (Actor|DestroyActor)))

(event EventBeginPlay
  (if (Variables|Default|GetAuto_Lancement)
    (bind _asbp_player (Utilities|Casting|CastToBP_Player (Game|GetPlayerCharacter 0)))
    (Default|CheckSON _asbp_player)
    (Components|Activation|Activate (Variables|Default|GetAudio) false)
    (Utilities|FlowControl|Delay 15.0)
    (if (not (Variables|Default|Getloop?))
      (Actor|DestroyActor))))

(fn ConstructionScript)